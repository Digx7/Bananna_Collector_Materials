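; BP_Banana is a banana actor in the BananaCollector game that spins in place with a randomized look.
; On BeginPlay it creates a dynamic material instance on its StaticMesh and randomizes the color multiplier and hue shift, so each banana varies.
; Tick rotates the actor around its local yaw axis by RotationSpeed scaled by delta time, keeping the spin frame-rate independent.
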(event EventBeginPlay
  (bind _returnvalue (Rendering|Material|CreateDynamicMaterialInstance (Variables|Default|GetStaticMesh) 0 0 "None" :!class /Script/Engine.PrimitiveComponent))
  (Variables|Default|SetBananaMaterial _returnvalue)
  (Rendering|Material|SetScalarParameterValue (Variables|Default|GetBananaMaterial) "ColorMultiplier" (Math|Random|RandomFloatinRange 0.0 5.0) :!class /Script/Engine.MaterialInstanceDynamic)
  (Rendering|Material|SetScalarParameterValue (Variables|Default|GetBananaMaterial) "HueShiftPercentage" (Math|Random|RandomFloatinRange 0.0 1e+02) :!class /Script/Engine.MaterialInstanceDynamic))

(event EventTick
  (params (DeltaSeconds :type Float%20%28single-precision%29))
  (Transformation|AddActorLocalRotation (Math|Rotator|MakeRotator 0.0 0.0 (* DeltaSeconds (Variables|Default|GetRotationSpeed))) false false))

(fn ConstructionScript)